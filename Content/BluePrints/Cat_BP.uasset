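; Clickable cat actor that meows, shows a new desire and gains saturation when its sprite is clicked.
; The CatSprite click event plays a 2D meow and sets DesireSprite to a random pick from five sprites.
; It then casts itself to Cat to read Saturation and raises it by a fixed amount.
; BeginPlay, Tick, overlap and a separate OnClicked binding are inactive stubs.
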(event OnClicked(CatSprite)
  (params (TouchedComponent :type Primitive%20Component%20Object%20Reference) (ButtonPressed :type Key%20Structure :default "None"))
  (Audio|PlaySound2D "/Game/Sounds/Meow.Meow" 1.0 1.0 0.0 0 0)
  (Rendering|Components|Sprite|SetSprite (Variables|Default|GetDesireSprite) (.OutItem (Utilities|Array|Random (Utilities|Array|MakeArray (Variables|Default|Getsprite_0) (Variables|Default|Getsprite_1) (Variables|Default|Getsprite_2) (Variables|Default|Getsprite_3) (Variables|Default|Getsprite_4)))))
  (bind _ascat (Utilities|Casting|CastToCat self))
  (bind _output_get (Variables|Default|SetSaturation (Variables|/Script/CatFeeder.Cat|GetSaturation _ascat)))
  (Variables|Default|SetSaturation (+ _output_get 3e+01)))

(event Custom|OnClicked_Event
  (params (TouchedActor :type Actor%20Object%20Reference) (ButtonPressed :type Key%20Structure :default "None")))

(event EventBeginPlay)

(event Collision|EventActorBeginOverlap
  (params (OtherActor :type Actor%20Object%20Reference)))

(event EventTick
  (params (DeltaSeconds :type Float%20%28single-precision%29)))

(fn ConstructionScript)